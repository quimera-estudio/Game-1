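; Interactable door frame Blueprint that the player opens and closes with the E key while standing in its trigger box.
; Box overlap begin and end events enable and disable input for player controller 0 on the actor.
; E checks the DoorRotation timeline's current angle to play it forward or reverse it.
; Each timeline update sets the Door's relative yaw, swinging it open or shut.
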(event `self.Box.OnComponentBeginOverlap`
  (params (OverlappedComponent :type "PrimitiveComponent Object Reference") (OtherActor :type "Actor Object Reference") (OtherComp :type "PrimitiveComponent Object Reference") (OtherBodyIndex :type Integer) (bFromSweep :type Boolean) (SweepResult :type "HitResult Structure (by ref)"))
  (`self.EnableInput` (`GameplayStatics.GetPlayerController` 0)))

(event `Key|E`
  (params (Key :type "Key Structure"))
  (:`Pressed`
    (if (< (stale _doorrotation) 1.0)
      (bind (_direction _doorrotation) (`Timeline|DoorRotation` :!label _label) ; Animação de abre e fecha
        (:`Update`
          (`SceneComponent.K2_SetRelativeRotation` (`self.Door`) (`KismetMathLibrary.MakeRotator` 0.0 0.0 _doorrotation) false false) ; OnUpdate da animação ele seta nova rotação para variável porta
        ))
      (else
        (goto _label :!via `Reverse`)))))

(event `self.Box.OnComponentEndOverlap`
  (params (OverlappedComponent :type "PrimitiveComponent Object Reference") (OtherActor :type "Actor Object Reference") (OtherComp :type "PrimitiveComponent Object Reference") (OtherBodyIndex :type Integer))
  (`self.DisableInput` (`GameplayStatics.GetPlayerController` 0)))

(fn `UserConstructionScript`)